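; Behavior tree task that picks the BP_FirstPersonCharacter with the lowest health as an AI target.
; On execute it scans all actors of that class, keeping any whose health is at or below LowestHealth, which the graph never resets.
; It writes the selected character's current location, as a vector rather than an actor reference, to BlackboardKey and succeeds, or fails without a valid selection.
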(event EventReceiveExecuteAI
  (params (OwnerController :type AI%20Controller%20Object%20Reference) (ControlledPawn :type Pawn%20Object%20Reference))
  (bind _outactors (Actor|GetAllActorsOfClass "/Game/FirstPerson/Blueprints/BP_FirstPersonCharacter.BP_FirstPersonCharacter_C"))
  (for _array_element _outactors
    (if (<= (Class|NetTestFPCharacter|GetHealth _array_element) (Variables|Default|GetLowestHealth))
      (Variables|Default|SetLowestHealth (Class|NetTestFPCharacter|GetHealth _array_element))
      (Variables|Default|SetSelectedCharacter _array_element)))
  (if (Utilities|IsValid (Variables|Default|GetSelectedCharacter))
    (AI|BehaviorTree|SetBlackboardValueasVector (Variables|Default|GetBlackboardKey) (Transformation|GetActorLocation (Variables|Default|GetSelectedCharacter)))
    (AI|BehaviorTree|FinishExecute true)
    (else
      (AI|BehaviorTree|FinishExecute false))))